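; BP_ScalingShape is an AutoTiler demo actor that shows a random primitive shape changing size over time.
; The construction script gives the Shape mesh a random cube, sphere, cone or cylinder and a random AutoTiler material instance.
; On BeginPlay it rescales immediately, then a looping timer periodically sets a random preset, mostly non-uniform world scale.
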(event `self.ReceiveBeginPlay`
  ;[1 1 1] Picks a random scale and intervals on a timer
  (`self.Scale Shape`)
  (`KismetSystemLibrary.K2_SetTimerDelegate` (delegate `Scale Shape`) 3.0 true))

(event `Scale Shape`
  ;[1 1 1] Picks a random scale and intervals on a timer
  (`SceneComponent.SetWorldScale3D` (`self.Shape`) (select `int` (`KismetMathLibrary.RandomInteger` 5) :`0` (1.0 1.0 1.0) :`1` (3.0 3.5 4.0) :`2` (5.0 4.0 5.0) :`3` (4.0 3.0 5.0) :`4` (6.0 8.0 5.0) :!type "Vector Structure")))

(fn `Set Shape Type`
  (`StaticMeshComponent.SetStaticMesh` (`self.Shape`) (select `int` (`KismetMathLibrary.RandomInteger` 4) :`0` "/Engine/BasicShapes/Cube.Cube" :`1` "/Engine/BasicShapes/Sphere.Sphere" :`2` "/Engine/BasicShapes/Cone.Cone" :`3` "/Engine/BasicShapes/Cylinder.Cylinder" :!type "StaticMesh Object Reference"))
  (`PrimitiveComponent.SetMaterial` (`self.Shape`) 0 (select `int` (`KismetMathLibrary.RandomInteger` 4) :`0` "/Game/AutoTiler/Materials/MI_AutoTiler_Grass.MI_AutoTiler_Grass" :`1` "/Game/AutoTiler/Materials/MI_AutoTiler_Rock.MI_AutoTiler_Rock" :`2` "/Game/AutoTiler/Materials/MI_AutoTiler_RockyMud.MI_AutoTiler_RockyMud" :`3` "/Game/AutoTiler/Materials/MI_AutoTiler_SheetMetal.MI_AutoTiler_SheetMetal" :!type "MaterialInterface Object Reference"))
  (return))

(fn `UserConstructionScript`
  (`self.Set Shape Type`))