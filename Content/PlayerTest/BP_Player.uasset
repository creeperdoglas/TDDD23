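; First-person parkour player character with jump, double jump, dash, smooth crouch, wallrun, walljump and grapple, mostly gated by saved ability flags.
; Tagged-wall overlaps drive timeline wallruns and camera tilt, while grappling line-traces and launches the player.
; A DoN jump counter and dash flag reset on landing, wallrun, grapple or bouncepad.
; Also handles footsteps, damage overlay, pause, save data and death, which respawns or restarts the escape level.
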(event `self.BP_OnDeath`
  (if (`self.IsEscaping`)
    (bind _asbp_gameinstance (cast `/Game/PlayerTest/BP_Building/Save/BP_Gameinstance` (`GameplayStatics.GetGameInstance`)))
    (`/Game/PlayerTest/BP_Building/Save/BP_Gameinstance.Stop Music Escape` _asbp_gameinstance)
    (`GameplayStatics.OpenLevelBySoftObjectPtr` "/Game/level/finalchallenge.finalchallenge")
    (set `self.IsEscaping` false)
    (set `self.HaveAbilityGrapple` false)
    (else
      (bind _asinput_gamemode (cast `/Game/PlayerTest/InputGamemode` (`GameplayStatics.GetGameMode`)))
      (`/Game/PlayerTest/InputGamemode.Set Player Spawn` _asinput_gamemode)))
  (`/Game/PlayerTest/BP_Building/UI/Loadingscreen/WB_LoadingScreen.LoadingAnim` (`self.WBLoad`) "Reverse")
  (set `self.Health` 100.0)
  ; HealthBar
  (`WidgetLayoutLibrary.RemoveAllWidgets` :!label _label)
  (bind _returnvalue (`|CreateWidget` "/Game/FirstPerson/Blueprints/BP_HealthBar_Widget.BP_HealthBar_Widget_C"))
  (`UserWidget.SetDesiredSizeInViewport` _returnvalue (300.0 30.0))
  (`UserWidget.SetAlignmentInViewport` _returnvalue (0.0 -35.0))
  (`UserWidget.SetAnchorsInViewport` :`self` _returnvalue)
  (`UserWidget.AddToViewport` _returnvalue 0)
  ; La till för att kunna köra Begin play igenpå annan plats
  (`self.Event Begin`)
  (bind _returnvalue_2 (`|CreateWidget` "/Game/PlayerTest/BP_Building/UI/Loadingscreen/WB_LoadingScreen.WB_LoadingScreen_C"))
  (bind _output_get (set `self.WBLoad` _returnvalue_2))
  (`/Game/PlayerTest/BP_Building/UI/Loadingscreen/WB_LoadingScreen.LoadingAnim` _output_get "Reverse")
  (`UserWidget.AddToViewport` _output_get 0)
  ; background ambiance stop
  (bind _asbp_gameinstance_2 (cast `/Game/PlayerTest/BP_Building/Save/BP_Gameinstance` (`GameplayStatics.GetGameInstance`)))
  (if (`self.IsEscaping`)
    (`/Game/PlayerTest/BP_Building/Save/BP_Gameinstance.StartEscape` _asbp_gameinstance_2)
    (else
      (`/Game/PlayerTest/BP_Building/Save/BP_Gameinstance.Play Music` _asbp_gameinstance_2 "/Game/Free_Sounds_Pack/cue/Exploration.Exploration")
      (`/Game/PlayerTest/BP_Building/Save/BP_Gameinstance.Stop Music` _asbp_gameinstance_2))))

(event `self.ReceiveBeginPlay`
  ; HealthBar
  (goto _label))

(event `Key|R`
  (params (Key :type "Key Structure"))
  ; Skapa variablerna i BP_Savegame också
  ;; Saving variables for player
  ;;; Test variabler för save
  (:`Pressed`
    (set `self.Gold` 15)
    (set `self.HaveAbilityDash` true)
    (set `self.HaveAbilityJump` true)
    (set `self.HaveAbilityDoubleJ` true)
    (set `self.HaveAbilityWallJ` true)
    (set `self.HaveAbilityWallR` true)
    (set `self.HaveAbilityGrapple` true)))

(event `/Game/PlayerTest/BP_Building/Save/BPI_Saveable.Save Data`
  (params (`Save Game Ref` :type "/Game/PlayerTest/BP_Building/Save/BP_SaveGame Object Reference"))
  ; Skapa variablerna i BP_Savegame också
  ;; Saving variables for player
  ;;; Test variabler för save
  (set `/Game/PlayerTest/BP_Building/Save/BP_SaveGame.Gold` (`self.Gold`) `Save Game Ref`)
  (set `/Game/PlayerTest/BP_Building/Save/BP_SaveGame.HaveAbilityDash` (`self.HaveAbilityDash`) `Save Game Ref`)
  (set `/Game/PlayerTest/BP_Building/Save/BP_SaveGame.HaveAbilityJump` (`self.HaveAbilityJump`) `Save Game Ref`)
  (set `/Game/PlayerTest/BP_Building/Save/BP_SaveGame.HaveAbilityDoubleJ` (`self.HaveAbilityDoubleJ`) `Save Game Ref`)
  (set `/Game/PlayerTest/BP_Building/Save/BP_SaveGame.HaveAbilityWallJ` (`self.HaveAbilityWallJ`) `Save Game Ref`)
  (set `/Game/PlayerTest/BP_Building/Save/BP_SaveGame.HaveAbilityWallR` (`self.HaveAbilityWallR`) `Save Game Ref`)
  (set `/Game/PlayerTest/BP_Building/Save/BP_SaveGame.HaveAbilityGrapple` (`self.HaveAbilityGrapple`) `Save Game Ref`)
  (set `/Game/PlayerTest/BP_Building/Save/BP_SaveGame.IsEscaping` (`self.IsEscaping`) `Save Game Ref`))

(event `self.BP_OnDamaged`
  (params (Damage :type "Float (single-precision)"))
  (bind _returnvalue (`|CreateWidget` "/Game/PlayerTest/RedOverlayImage.RedOverlayImage_C"))
  (`UserWidget.AddToViewport` _returnvalue 0)
  (`KismetSystemLibrary.K2_SetTimerDelegate` (delegate `HideOverlay`) 0.3))

(event `InputAction|Pause` :paused true
  (params (Key :type "Key Structure"))
  (bind _returnvalue (`GameplayStatics.GetPlayerController` 0))
  ; Pause and unpause
  (:`Pressed`
    (if (not (`self.IsPause`))
      (set `self.IsPause` true)
      (bind _returnvalue_2 (`|CreateWidget` "/Game/PlayerTest/BP_Building/UI/Menu/WB_Pausemenu.WB_Pausemenu_C" _returnvalue))
      (bind _output_get (set `self.Pause Menu Widget` _returnvalue_2))
      (`UserWidget.AddToViewport` _output_get 0)
      (`WidgetBlueprintLibrary.SetInputMode_GameAndUIEx` _returnvalue null)
      (set `PlayerController.bShowMouseCursor` true (`GameplayStatics.GetPlayerController` 0))
      (`GameplayStatics.SetGamePaused` true)
      (else
        (set `self.IsPause` false)
        (`Widget.RemoveFromParent` (`self.Pause Menu Widget`))
        (`GameplayStatics.SetGamePaused` false)
        (`WidgetBlueprintLibrary.SetInputMode_GameOnly` _returnvalue)
        (set `PlayerController.bShowMouseCursor` false (`GameplayStatics.GetPlayerController` 0))))))

(event `self.Footstep.OnAudioFinished`
  ; Adding footsteps
  (if (!= (`NavMovementComponent.GetVelocityForNavMovement` (`self.CharacterMovement`)) (0.0 0.0 0.0))
    (if (and (`self.Check movement`) (not (`NavMovementComponent.IsFalling` (`self.CharacterMovement`)))) :!label _label_2
      (`AudioComponent.Play` (`self.Footstep`) 0.0 :!label _label_3)
      (elif (`self.IsWallrunning`)
        (goto _label_3)
        (else
          (set `self.Check movement` false))))))

(event `HideOverlay`
  (`Widget.RemoveFromParent` (stale `self.BP_OnDamaged` _returnvalue)))

(event `/Game/PlayerTest/BP_Building/Save/BPI_Saveable.Load Data`
  (params (`Save Game Ref` :type "/Game/PlayerTest/BP_Building/Save/BP_SaveGame Object Reference"))
  ; Skapa variablerna i BP_Savegame också
  ;; Saving variables for player
  ;;; Test variabler för save
  (set `self.Gold` (`/Game/PlayerTest/BP_Building/Save/BP_SaveGame.Gold` `Save Game Ref`))
  (set `self.HaveAbilityDash` (`/Game/PlayerTest/BP_Building/Save/BP_SaveGame.HaveAbilityDash` `Save Game Ref`))
  (set `self.HaveAbilityJump` (`/Game/PlayerTest/BP_Building/Save/BP_SaveGame.HaveAbilityJump` `Save Game Ref`))
  (set `self.HaveAbilityDoubleJ` (`/Game/PlayerTest/BP_Building/Save/BP_SaveGame.HaveAbilityDoubleJ` `Save Game Ref`))
  (set `self.HaveAbilityWallJ` (`/Game/PlayerTest/BP_Building/Save/BP_SaveGame.HaveAbilityWallJ` `Save Game Ref`))
  (set `self.HaveAbilityWallR` (`/Game/PlayerTest/BP_Building/Save/BP_SaveGame.HaveAbilityWallR` `Save Game Ref`))
  (set `self.HaveAbilityGrapple` (`/Game/PlayerTest/BP_Building/Save/BP_SaveGame.HaveAbilityGrapple` `Save Game Ref`))
  (set `self.IsEscaping` (`/Game/PlayerTest/BP_Building/Save/BP_SaveGame.IsEscaping` `Save Game Ref`)))

(event `Key|W`
  (params (Key :type "Key Structure"))
  ; Adding footsteps
  (:`Pressed`
    (set `self.Check movement` true :!label _label_4)
    (goto _label_2)))

(event `Key|S`
  (params (Key :type "Key Structure"))
  ; Adding footsteps
  (:`Pressed`
    (goto _label_4)))

(event `Onlanding`
  ; Adding footsteps
  (set `self.Check movement` true)
  (goto _label_3))

(event `Key|A`
  (params (Key :type "Key Structure"))
  ; Adding footsteps
  (:`Pressed`
    (goto _label_4)))

(event `Key|D`
  (params (Key :type "Key Structure"))
  ; Adding footsteps
  (:`Pressed`
    (goto _label_4)))

(event `Event Begin`
  (bind _charactermovement (`self.CharacterMovement`))
  ; Player Movement
  ;; Sets old Variables to get later and request load
  (`MovementComponent.SetPlaneConstraintEnabled` (`self.CharacterMovement`) true)
  (set `self.Old Gravity Scale` (`CharacterMovementComponent.GravityScale` _charactermovement))
  (set `self.Old Capsule Half Height` (`CapsuleComponent.CapsuleHalfHeight` (`self.CapsuleComponent`)))
  (set `self.OldWalkingSpeed` (`CharacterMovementComponent.MaxWalkSpeed` _charactermovement))
  (set `self.OldFriction` (`CharacterMovementComponent.FallingLateralFriction` _charactermovement))
  (message `/Game/PlayerTest/BP_Building/Save/BPI_Persistance.Request Load` (`GameplayStatics.GetGameInstance`) self))

(event `InputAxis|Rotate`
  (params (AxisValue :type "Float (single-precision)"))
  ; Player Movement
  ;; Camera
  (`self.AddControllerYawInput` AxisValue))

(event `InputAxis|Forward`
  (params (AxisValue :type "Float (single-precision)"))
  ; Player Movement
  ;; Base movement
  (`self.AddMovementInput` (`SceneComponent.GetForwardVector` (`self.CapsuleComponent`)) AxisValue))

(event `self.UncrouchCapsule.OnComponentBeginOverlap`
  (params (OverlappedComponent :type "PrimitiveComponent Object Reference") (OtherActor :type "Actor Object Reference") (OtherComp :type "PrimitiveComponent Object Reference") (OtherBodyIndex :type Integer) (bFromSweep :type Boolean) (SweepResult :type "HitResult Structure (by ref)"))
  ; Player Movement
  ;; Check for overlaps above when crouching
  ;;; Put checkpoint on lower half of player
  (if (!= OtherActor self)
    (`/Engine/EditorBlueprintResources/StandardMacros.IncrementInt` (`self.UnCrouchOverlapCount`))))

(event `Lose one jump`
  ; Player Movement
  ;; Action Jump and  Double jump
  ;;; Inc when dropping off wall/or bouncpad usage
  (bind _counter (`/Engine/EditorBlueprintResources/StandardMacros.Do N` 2 :!label _label_5)
    (:`Exit`
      (switch `int` _counter
        (:`1`
          (if (`self.IsWallrunning`) :!label _label_6
            (`|ExecutionSequence`
              (:`then_0`
                (set `self.NotJumped` false))
              (:`then_1`
                (`self.Jump Off Wall`)))
            (else
              (`self.LaunchCharacter` (0.0 0.0 800.0) false true))))
        (:`2`
          (`AudioComponent.Play` (`self.DoubleSFX`) 0.0)
          (if (`self.HaveAbilityDoubleJ`)
            (goto _label_6)))))))

(event `InputAxis|lookup`
  (params (AxisValue :type "Float (single-precision)"))
  ; Player Movement
  ;; Camera
  (`self.AddControllerPitchInput` AxisValue))

(event `InputAction|Jump`
  (params (Key :type "Key Structure"))
  ; Player Movement
  ;; Action Jump and  Double jump
  (:`Pressed`
    (`|ExecutionSequence`
      (:`then_0`
        (if (`self.HaveAbilityJump`)
          (goto _label_5)))
      (:`then_1`
        ;;; Edgecase logic
        ;;; Needed if we want to not be able to jump an additional time in the air if we dash off of a ledge without jumping
        (if (and (`self.NotJumped`) (`NavMovementComponent.IsFalling` (`self.CharacterMovement`)))
          (`self.Lose one jump`))))))

(event `InputAxis|Right`
  (params (AxisValue :type "Float (single-precision)"))
  ; Player Movement
  ;; Base movement
  (`self.AddMovementInput` (`SceneComponent.GetRightVector` (`self.CapsuleComponent`)) AxisValue))

(event `dash in air`
  ; Dash only once in air
  (if (== (`NavMovementComponent.IsFalling` (`self.CharacterMovement`)) (`self.isDashing`))
    (set `self.Has AirDashed` true)))

(event `self.UncrouchCapsule.OnComponentEndOverlap`
  (params (OverlappedComponent :type "PrimitiveComponent Object Reference") (OtherActor :type "Actor Object Reference") (OtherComp :type "PrimitiveComponent Object Reference") (OtherBodyIndex :type Integer))
  ; Player Movement
  ;; Check for overlaps above when crouching
  ;;; Put checkpoint on lower half of player
  (if (!= OtherActor self)
    (`/Engine/EditorBlueprintResources/StandardMacros.DecrementInt` (`self.UnCrouchOverlapCount`))))

(event `InputAction|Crouch`
  (params (Key :type "Key Structure"))
  ; Player Movement
  ;; Action Smooth Crouch
  (:`Pressed`
    (`self.Start Crouch`))
  (:`Released`
    (`self.End Crouch`)))

(event `Reset Jump`
  ; Player Movement
  ;; Action Jump and  Double jump
  ;;; Reset doublejump on wallrun
  (goto _label_5 :!via `Reset`))

(event `self.OnLanded`
  (params (Hit :type "HitResult Structure (by ref)"))
  ; Player Movement
  ;; Action Jump and  Double jump
  (`self.Reset Dash`)
  (`self.Onlanding`)
  (`self.Reset Speed`)
  (`|ExecutionSequence`
    (:`then_0`
      (goto _label_5 :!via `Reset`))
    (:`then_1`
      (set `self.NotJumped` true))))

(event `Reset Dash`
  ; Dash only once in air
  (set `self.Has AirDashed` false))

(event `Start Crouch`
  ; Player Movement
  ;; Action Smooth Crouch
  (bind (_direction _alpha) (`Timeline|Crouch Timline` :!label _label_7)
    (:`Update`
      (`CapsuleComponent.SetCapsuleHalfHeight` (`self.CapsuleComponent`) (`KismetMathLibrary.Lerp` (`self.Old Capsule Half Height`) (`CharacterMovementComponent.CrouchedHalfHeight` (`self.CharacterMovement`)) _alpha) true))
    (:`Finished`
      (if (`|EnumEquality` _direction "Forward")
        (`self.Crouch`)
        (else
          (`self.UnCrouch`))))))

(event `InputAction|Dash`
  (params (Key :type "Key Structure"))
  (bind (_returnvalue_x _returnvalue_y) (`KismetMathLibrary.BreakVector` (* (`self.GetVelocity`) 20.0)))
  ; Player Movement
  ;; Experimental dash
  (:`Pressed`
    (if (`self.HaveAbilityDash`)
      (if (`self.Has AirDashed`)
        _
        (elif (not (`self.isDashing`))
          (set `self.isDashing` true)
          (`AudioComponent.Play` (`self.DashSFX`) 0.0)
          (`self.LaunchCharacter` (`KismetMathLibrary.MakeVector` _returnvalue_x _returnvalue_y 1.0) false true)
          (`self.dash in air`)
          (`KismetSystemLibrary.Delay` 1.0)
          (set `self.isDashing` false))))))

(event `self.ReceiveTick`
  (params (DeltaSeconds :type "Float (single-precision)"))
  ; Player Movement
  ;; Check for overlaps above when crouching
  ;;; Improved Uncrouch logic
  (`|ExecutionSequence`
    (:`then_0`
      (set `self.Delta Seconds` DeltaSeconds))
    (:`then_1`
      (if (and (<= (`self.UnCrouchOverlapCount`) 0) (`self.WantUncrouch`))
        (set `self.WantUncrouch` false)
        (set `self.UnCrouchOverlapCount` 0)
        (`self.Do Uncrouch`)))))

(event `Reset Speed`
  (set `CharacterMovementComponent.MaxWalkSpeed` (`self.OldWalkingSpeed`) (`self.CharacterMovement`)))

(event `Do Uncrouch`
  ; Player Movement
  ;; Action Smooth Crouch
  (goto _label_7 :!via `Reverse`))

(event `End Crouch`
  ; Player Movement
  ;; Action Smooth Crouch
  (set `self.WantUncrouch` true))

(event `Reset Air Decel`
  (set `CharacterMovementComponent.FallingLateralFriction` (`self.OldFriction`) (`self.CharacterMovement`)))

(event `self.DetectWallCapsule.OnComponentBeginOverlap`
  (params (OverlappedComponent :type "PrimitiveComponent Object Reference") (OtherActor :type "Actor Object Reference") (OtherComp :type "PrimitiveComponent Object Reference") (OtherBodyIndex :type Integer) (bFromSweep :type Boolean) (SweepResult :type "HitResult Structure (by ref)"))
  (bind _returnvalue (`self.GetActorForwardVector` OtherActor))
  (bind _charactermovement (`self.CharacterMovement`))
  (bind _returnvalue_2 (`KismetMathLibrary.Dot_VectorVector` _returnvalue (`SceneComponent.GetForwardVector` (`self.Camera`))))
  ; Player Movement
  ;; Wallrun
  (if (or (`self.HaveAbilityWallR`) (`self.HaveAbilityWallJ`))
    (if (and (`self.ActorHasTag` OtherActor "WallRun") (`NavMovementInterface.IsFalling` (`self.CharacterMovement`)))
      (set `self.Wall` OtherActor)
      (`|ExecutionSequence`
        (:`then_0`
          (`self.Reset Jump`))
        (:`then_1`
          (set `self.IsWallrunning` true)
          (set `self.PlayerDirection` (* _returnvalue (+ (`KismetMathLibrary.SelectInt` 1 0 (> _returnvalue_2 0.5)) (`KismetMathLibrary.SelectInt` -1 0 (< _returnvalue_2 -0.5)))))
          (`MovementComponent.SetPlaneConstraintNormal` (`self.CharacterMovement`) (0.0 0.0 0.0))
          (set `CharacterMovementComponent.GravityScale` 0.0 (`self.CharacterMovement`))
          (`self.Onlanding`)
          (`Timeline|WallRun Timeline` :!via `PlayFromStart` :!label _label_8
            (:`Update`
              (`self.Reset Dash`)
              (if (`self.HaveAbilityWallR`)
                (set `CharacterMovementComponent.MaxWalkSpeed` 1500.0 _charactermovement)
                (set `MovementComponent.Velocity` (* (`self.PlayerDirection`) 3000.0) (`self.CharacterMovement`))
                (else
                  (set `MovementComponent.Velocity` (* (`self.PlayerDirection`) 0.01) _charactermovement))))
            (:`Finished`
              ;;; Ending Wallrun
              (`MovementComponent.SetPlaneConstraintNormal` (`self.CharacterMovement`) (0.0 0.0 0.0))
              (set `self.IsWallrunning` false)
              (set `CharacterMovementComponent.GravityScale` (`self.Old Gravity Scale`) (`self.CharacterMovement`))
              (`self.Lose one jump`)
              ;;;; Movement launiching off the wall when finished
              (`self.LaunchCharacter` (0.0 0.0 300.0) :!label _label_9))))))))

(event `InputAction|Grapple`
  (params (Key :type "Key Structure"))
  (bind _returnvalue (`self.K2_GetActorLocation`))
  ; Player Movement
  ;; Grappling
  ;;; Start Grapple
  (:`Pressed`
    (if (`self.HaveAbilityGrapple`)
      (if (`self.CanGrapple`)
        ;;;; Target and Direction for grapple
        (set `self.CanGrapple` false)
        (set `self.IsGrappling` true)
        (set `CharacterMovementComponent.GravityScale` 1.0 (`self.CharacterMovement`))
        (bind (_outhit _returnvalue_2) (`KismetSystemLibrary.LineTraceSingle` _returnvalue (+ _returnvalue (* (`SceneComponent.GetForwardVector` (`self.Camera`)) (`self.GrappleDistance`))) "TraceTypeQuery2"))
        ;;;; Grapple to target
        (if _returnvalue_2
          (set `self.GrappleLocation` (`.Location` (`GameplayStatics.BreakHitResult` _outhit)))
          (`self.ShootGrapple`)
          (`self.LaunchCharacter` (0.0 0.0 500.0) true true)
          (`KismetSystemLibrary.Delay` 0.0)
          (`self.Reset Jump`)
          (`self.Lose one jump`)
          (set `CharacterMovementComponent.FallingLateralFriction` 0.0 (`self.CharacterMovement`))
          (`self.LaunchCharacter` (* (- (`self.GrappleLocation`) (`self.K2_GetActorLocation`)) 2.5) true)
          (`self.Reset Dash`)
          (else
            (`self.Reset Grapple`)))))))

(event `Stop Wallrun TImeLine`
  ; Player Movement
  ;; Wallrun
  (goto _label_8 :!via `Stop`))

(event `self.DetectWallCapsule.OnComponentEndOverlap`
  (params (OverlappedComponent :type "PrimitiveComponent Object Reference") (OtherActor :type "Actor Object Reference") (OtherComp :type "PrimitiveComponent Object Reference") (OtherBodyIndex :type Integer))
  ; Player Movement
  ;; Wallrun
  ;;; Ending Wallrun
  (set `self.Wall` null)
  (if (`self.ActorHasTag` OtherActor "Wallrun")
    (`|ExecutionSequence`
      (:`then_0`
        (goto _label_8 :!via `Stop`))
      (:`then_1`
        (`MovementComponent.SetPlaneConstraintNormal` (`self.CharacterMovement`) (0.0 0.0 0.0))
        (set `self.IsWallrunning` false)
        (set `CharacterMovementComponent.GravityScale` (`self.Old Gravity Scale`) (`self.CharacterMovement`))
        (goto _label_9)))))

(event `Reset Grapple`
  (bind _charactermovement (`self.CharacterMovement`))
  ; Player Movement
  ;; Grappling
  ;;; Reset Grapple Event
  (`SceneComponent.SetVisibility` (`self.GrappleCable`) false false)
  (if (not (`self.IsWallrunning`))
    (set `CharacterMovementComponent.GravityScale` (`self.Old Gravity Scale`) _charactermovement))
  (set `self.IsGrappling` false)
  (`KismetSystemLibrary.Delay` 0.2)
  (set `CharacterMovementComponent.FallingLateralFriction` (`self.OldFriction`) _charactermovement)
  (`KismetSystemLibrary.Delay` (`self.GrappleCooldown`))
  (set `self.CanGrapple` true))

(event `ShootGrapple`
  ; Player Movement
  ;; Grappling
  ;;; Shoot grapplehook event
  (`AudioComponent.Play` (`self.Grapple`) 0.0)
  (`SceneComponent.SetVisibility` (`self.GrappleCable`) true false)
  (bind (_direction _interp_speed) (`Timeline|Grapple Timeline` :!via `PlayFromStart`)
    (:`Update`
      (`SceneComponent.K2_SetWorldLocation` (`self.GrappleCable`) (`KismetMathLibrary.VInterpTo` (`SceneComponent.K2_GetComponentLocation` (`self.GrappleCable`)) (`self.GrappleLocation`) (`self.Delta Seconds`) _interp_speed) false false)
      (`KismetSystemLibrary.Delay` 0.2)
      (`self.Reset Grapple`))))

(event `self.WallDetectRight.OnComponentBeginOverlap`
  (params (OverlappedComponent :type "PrimitiveComponent Object Reference") (OtherActor :type "Actor Object Reference") (OtherComp :type "PrimitiveComponent Object Reference") (OtherBodyIndex :type Integer) (bFromSweep :type Boolean) (SweepResult :type "HitResult Structure (by ref)"))
  (bind _returnvalue_roll (`KismetMathLibrary.BreakRotator` (`self.K2_GetActorRotation`)))
  (bind _returnvalue (`GameplayStatics.GetPlayerController` 0))
  (bind (_returnvalue_roll_2 _returnvalue_pitch _returnvalue_yaw) (`KismetMathLibrary.BreakRotator` (`Controller.GetControlRotation` _returnvalue)))
  ; Player Movement
  ;; Wallrun
  ;;; Rotate Camera Right on Left wall
  (if (and (`self.ActorHasTag` OtherActor "WallRun") (`NavMovementComponent.IsFalling` (`self.CharacterMovement`)))
    (bind (_direction _alpha) (`Timeline|RotateCameraRightTimeline` :!label _label_10)
      (:`Update`
        (`Controller.SetControlRotation` _returnvalue (`KismetMathLibrary.MakeRotator` (`KismetMathLibrary.Lerp` _returnvalue_roll -5.0 _alpha) _returnvalue_pitch _returnvalue_yaw))))))

(event `self.WallDetectLeft.OnComponentBeginOverlap`
  (params (OverlappedComponent :type "PrimitiveComponent Object Reference") (OtherActor :type "Actor Object Reference") (OtherComp :type "PrimitiveComponent Object Reference") (OtherBodyIndex :type Integer) (bFromSweep :type Boolean) (SweepResult :type "HitResult Structure (by ref)"))
  (bind _returnvalue_roll (`KismetMathLibrary.BreakRotator` (`self.K2_GetActorRotation`)))
  (bind _returnvalue (`GameplayStatics.GetPlayerController` 0))
  (bind (_returnvalue_roll_2 _returnvalue_pitch _returnvalue_yaw) (`KismetMathLibrary.BreakRotator` (`Controller.GetControlRotation` _returnvalue)))
  ; Player Movement
  ;; Wallrun
  ;;; Rotate Camerta Left on right wall
  (if (and (`self.ActorHasTag` OtherActor "WallRun") (`NavMovementComponent.IsFalling` (`self.CharacterMovement`)))
    (bind (_direction _alpha) (`Timeline|RotateCameraLeftTimeline` :!label _label_11)
      (:`Update`
        (`Controller.SetControlRotation` _returnvalue (`KismetMathLibrary.MakeRotator` (`KismetMathLibrary.Lerp` _returnvalue_roll 5.0 _alpha) _returnvalue_pitch _returnvalue_yaw))))))

(event `self.CapsuleComponent.OnComponentHit`
  (params (HitComponent :type "PrimitiveComponent Object Reference") (OtherActor :type "Actor Object Reference") (OtherComp :type "PrimitiveComponent Object Reference") (NormalImpulse :type "Vector Structure") (Hit :type "HitResult Structure (by ref)"))
  ; Player Movement
  ;; Grappling
  ;;; Little climb on grappling into object
  (if (`SceneComponent.IsSimulatingPhysics` OtherComp "None")
    _
    (elif (`self.IsGrappling`)
      (`self.LaunchCharacter` (0.0 0.0 600.0) true true))))

(event `self.WallDetectLeft.OnComponentEndOverlap`
  (params (OverlappedComponent :type "PrimitiveComponent Object Reference") (OtherActor :type "Actor Object Reference") (OtherComp :type "PrimitiveComponent Object Reference") (OtherBodyIndex :type Integer))
  ; Player Movement
  ;; Wallrun
  ;;; Rotate Camerta Left on right wall
  (if (`self.ActorHasTag` OtherActor "WallRun")
    (goto _label_11 :!via `Reverse`)))

(event `self.WallDetectRight.OnComponentEndOverlap`
  (params (OverlappedComponent :type "PrimitiveComponent Object Reference") (OtherActor :type "Actor Object Reference") (OtherComp :type "PrimitiveComponent Object Reference") (OtherBodyIndex :type Integer))
  ; Player Movement
  ;; Wallrun
  ;;; Rotate Camera Right on Left wall
  (if (`self.ActorHasTag` OtherActor "WallRun")
    (goto _label_10 :!via `Reverse`)))

(event `self.CapsuleComponent.OnComponentBeginOverlap`
  (params (OverlappedComponent :type "PrimitiveComponent Object Reference") (OtherActor :type "Actor Object Reference") (OtherComp :type "PrimitiveComponent Object Reference") (OtherBodyIndex :type Integer) (bFromSweep :type Boolean) (SweepResult :type "HitResult Structure (by ref)"))
  ; Player Movement
  ;; Grappling
  ;;; Only one jump in air after bouncepad
  (if (`ActorComponent.ComponentHasTag` OtherComp "Bouncepad")
    (`self.Reset Dash`)
    (`self.Reset Jump`)
    (`self.Lose one jump`)))

(event `Jump Off Wall`
  ; Player Movement
  ;; Wallrun
  ;;; WallJump During Run
  (if (`self.HaveAbilityWallJ`)
    (if (`self.IsWallrunning`)
      (`/Engine/EditorBlueprintResources/StandardMacros.IsValid` (`self.Wall`)
        (:`Is Valid`
          (bind _aswall_for_run (cast `/Game/PlayerTest/BP_Building/Wall/WallForRun` (`self.Wall`)))
          (`self.Stop Wallrun TImeLine`)
          (bind _returnvalue (`SceneComponent.GetForwardVector` (`/Game/PlayerTest/BP_Building/Wall/WallForRun.Arrow Right` _aswall_for_run)))
          (bind (_returnvalue_x _returnvalue_y) (`KismetMathLibrary.BreakVector` (* (* _returnvalue (`KismetMathLibrary.SelectInt` 1 -1 (> (`KismetMathLibrary.Dot_VectorVector` _returnvalue (- (`self.K2_GetActorLocation`) (`self.K2_GetActorLocation` (`self.Wall`)))) 0.0))) 3000)))
          (`self.LaunchCharacter` (`KismetMathLibrary.MakeVector` _returnvalue_x _returnvalue_y 1000.0) false true))))))

(fn `Dash`)

(fn `UserConstructionScript`)