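; Hazard volume that damages the player on overlap and handles death.
; Each overlap subtracts health, launches the player upward and flashes a red overlay widget, created at BeginPlay, removed by a short timer.
; At zero health an escaping player stops the escape music, loses grapple and reloads the Finalchallenge level.
; Otherwise the game mode respawns the player and health is restored to full.
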(event `self.ReceiveBeginPlay`
  (bind _returnvalue (`|CreateWidget` "/Game/PlayerTest/RedOverlayImage.RedOverlayImage_C"))
  (set `self.Dam` _returnvalue))

(event `self.Box.OnComponentBeginOverlap`
  (params (OverlappedComponent :type "PrimitiveComponent Object Reference") (OtherActor :type "Actor Object Reference") (OtherComp :type "PrimitiveComponent Object Reference") (OtherBodyIndex :type Integer) (bFromSweep :type Boolean) (SweepResult :type "HitResult Structure (by ref)"))
  ; Respawns player at nearest checkpoint
  (bind _asbp_player (cast `/Game/PlayerTest/BP_Player` OtherActor))
  (bind _asinput_gamemode (cast `/Game/PlayerTest/InputGamemode` (`GameplayStatics.GetGameMode`)))
  (bind _health (`InputCharacter.Health` _asbp_player))
  (set `InputCharacter.Health` (- _health 9.9) _asbp_player)
  (`Character.LaunchCharacter` _asbp_player (0.0 0.0 600.0) false true)
  (`UserWidget.AddToViewport` (`self.Dam`) 0)
  (`KismetSystemLibrary.K2_SetTimerDelegate` (delegate `Hide`) 0.3)
  (if (<= _health 0.0)
    (if (`/Game/PlayerTest/BP_Player.IsEscaping` _asbp_player)
      (bind _asbp_gameinstance (cast `/Game/PlayerTest/BP_Building/Save/BP_Gameinstance` (`GameplayStatics.GetGameInstance`)))
      (`/Game/PlayerTest/BP_Building/Save/BP_Gameinstance.Stop Music Escape` _asbp_gameinstance)
      (`GameplayStatics.OpenLevelBySoftObjectPtr` "/Game/level/finalchallenge.finalchallenge")
      (set `/Game/PlayerTest/BP_Player.IsEscaping` false _asbp_player)
      (set `/Game/PlayerTest/BP_Player.HaveAbilityGrapple` false _asbp_player)
      (else
        (`/Game/PlayerTest/InputGamemode.Set Player Spawn` _asinput_gamemode)
        (set `InputCharacter.Health` 100.0 _asbp_player)))))

(event `Hide`
  (`Widget.RemoveFromParent` (`self.Dam`)))

(fn `UserConstructionScript`)