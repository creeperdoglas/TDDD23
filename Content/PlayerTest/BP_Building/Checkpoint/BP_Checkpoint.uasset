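; BP_Checkpoint is a checkpoint actor that registers a respawn point when BP_Player enters its box collider.
; If inactive on entry, it turns active and passes its location, rotation, active flag and current level name to InputGamemode's SetCheckpoint.
; If already active, entry only clears the flag, and leaving the box always sets it active again as a noted bug workaround.
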(event `self.Box.OnComponentBeginOverlap`
  (params (OverlappedComponent :type "PrimitiveComponent Object Reference") (OtherActor :type "Actor Object Reference") (OtherComp :type "PrimitiveComponent Object Reference") (OtherBodyIndex :type Integer) (bFromSweep :type Boolean) (SweepResult :type "HitResult Structure (by ref)"))
  (bind (_returnvalue_location _returnvalue_rotation) (`KismetMathLibrary.BreakTransform` (`self.GetTransform`)))
  ; Checkpoint set when entering box collider (Added stuff in event begeinplay in gamemode)
  (cast `/Game/PlayerTest/BP_Player` OtherActor)
  (if (`self.Is Active`)
    (set `self.Is Active` false)
    (else
      (set `self.Is Active` true)
      (bind _asinput_gamemode (cast `/Game/PlayerTest/InputGamemode` (`GameplayStatics.GetGameMode`)))
      (bind _returnvalue (`GameplayStatics.GetCurrentLevelName` true))
      (`/Game/PlayerTest/InputGamemode.Set Checkpoint` _asinput_gamemode _returnvalue_location _returnvalue_rotation (`self.Is Active`) _returnvalue))))

(event `self.Box.OnComponentEndOverlap`
  (params (OverlappedComponent :type "PrimitiveComponent Object Reference") (OtherActor :type "Actor Object Reference") (OtherComp :type "PrimitiveComponent Object Reference") (OtherBodyIndex :type Integer))
  ; Bandaid for Refreshed checkpoint to count to avoid potential bugs
  (cast `/Game/PlayerTest/BP_Player` OtherActor)
  (set `self.Is Active` true))

(fn `UserConstructionScript`)